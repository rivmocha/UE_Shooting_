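; Player state for the shooting game, holding each player's HP, armor, name, kills and deaths.
; Setter functions change these values, and their OnRep handlers broadcast event dispatchers so listeners update without direct references.
; Armor absorbs damage until depleted; a hit that depletes it zeroes armor, then subtracts the full damage from HP.
; On BeginPlay it registers itself with the local player's shooting HUD for binding.
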(event EventBeginPlay
  (Development|PrintString (Utilities|String|Append "Create" (Utilities|GetDisplayName self) "..." "..." "..." "Pawn" (Utilities|GetDisplayName (Variables|Default|GetPawnPrivate))) true true "(R=1.000000,G=0.372432,B=0.000000,A=1.000000)" 1e+01)
  (CallFunction|InitBind))

(fn ConstructionScript)

(fn AddDamage
  (params (Damage :type Float%20%28single-precision%29))
  (if (> (- (Variables|Default|GetArmor) Damage) 0.0)
    (Variables|Default|SetArmor (- (Variables|Default|GetArmor) Damage))
    (else
      (Variables|Default|SetArmor 0.0)
      (bind _output_get (Variables|Default|SetHP (Math|Float|Clamp(Float) (+ (Variables|Default|GetHP) (- (Variables|Default|GetArmor) Damage)) 0.0 1e+02)))
      (Development|PrintString (Utilities|String|Append "Add damage result" (Utilities|String|ToString(Float) _output_get)) true false "(R=0.000000,G=0.660000,B=1.000000,A=1.000000)" 1e+01))))

(fn OnRepHP
  ;[1 1 1] Client
  (Development|PrintString (Utilities|String|Append "On Rep HP" (Utilities|String|ToString(Float) (Variables|Default|GetHP))) false false "(R=0.000000,G=0.660000,B=1.000000,A=1.000000)" 1e+01)
  (Default|CallEventDispatcherHP (Variables|Default|GetHP) (Variables|Default|GetMax%20HP)))

(fn AddHeal
  (params (Heal :type Float%20%28single-precision%29))
  (Variables|Default|SetHP (Math|Float|Clamp(Float) (+ (Variables|Default|GetHP) Heal) 0.0 1e+02)))

(fn OnRepArmor
  (Default|CallEventDispatcherArmor (Variables|Default|GetArmor) 1e+02))

(fn AddArmor
  (params (Armor :type Float%20%28single-precision%29))
  (Variables|Default|SetArmor (Math|Float|Clamp(Float) (+ (Variables|Default|GetArmor) Armor) 0.0 1e+02)))

(fn SetName
  (params (Name :type String))
  (Variables|Default|SetName Name))

(fn OnRepName
  (Development|PrintString (Utilities|String|Append "OnRepName" "   :   " (Variables|Default|GetName)) true true "(R=1.000000,G=0.216980,B=0.000000,A=1.000000)" 6e+01)
  (Default|CallEventDispatcherChangeName (Variables|Default|GetName)))

(fn InitBind
  (bind _asbp_shooting_hud (Utilities|Casting|CastToBP_ShootingHUD (HUD|GetHUD (Game|GetPlayerController 0)))
    (:then
      (Default|BindMyPlayerState _asbp_shooting_hud)
      (Default|BindPlayerState _asbp_shooting_hud self))
    (:CastFailed
      (Development|PrintString "ShootingHUD_Cast Fail" true true "(R=1.000000,G=0.025870,B=0.000000,A=1.000000)" 6e+01))))

(fn AddKill
  (Variables|Default|SetKill (+ (Variables|Default|GetKill) 1)))

(fn OnRepKill
  (Default|CallEventDispatcherKill (Variables|Default|GetKill)))

(fn OnRepDeath
  (Default|CallEventDispatcherDeath (Variables|Default|GetDeath)))

(fn AddDeath
  (Variables|Default|SetDeath (+ (Variables|Default|GetDeath) 1)))

(fn IsDeath
  (return (<= (Variables|Default|GetHP) 0.0)))