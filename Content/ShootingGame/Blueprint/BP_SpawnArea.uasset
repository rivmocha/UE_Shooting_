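; BP_SpawnArea is an item spawn point that keeps a random item available at its location in the shooting game.
; On BeginPlay, SpawnItem picks a random class from Items, spawns it at the area's transform and binds to its OnDestroyed event.
; The DestroyedItem handler sets a short timer that calls SpawnItem by name, forming a respawn loop.
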(event EventBeginPlay
  (CallFunction|SpawnItem))

(event Collision|EventActorBeginOverlap
  (params (OtherActor :type Actor%20Object%20Reference)))

(event EventTick
  (params (DeltaSeconds :type Float%20%28single-precision%29)))

(fn ConstructionScript)

(fn SpawnItem
  (Networking|SwitchHasAuthority
    (:Authority
      _)
    (:Remote
      _))
  (bind _returnvalue (Game|SpawnActorfromClass (.OutItem (Utilities|Array|Random (Variables|Default|GetItems))) (Transformation|GetActorTransform) "Undefined" 0 0))
  (bind _output_get (Variables|Default|SetSpawned_Item _returnvalue))
  (Utilities|IsValid _output_get
    (:Is%20Valid
      (Game|BindEventtoOnDestroyed _output_get (EventDispatchers|CreateEvent :!event DestroyedItem)))))

(fn DestroyedItem
  (params (DestroyedActor :type Actor%20Object%20Reference))
  (Utilities|Time|SetTimerbyFunctionName 0 "SpawnItem" 3.0))