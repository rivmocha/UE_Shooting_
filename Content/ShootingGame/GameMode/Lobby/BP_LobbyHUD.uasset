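; Lobby HUD that creates the lobby widget on BeginPlay and switches the player to UI-only input with a visible cursor.
; BindUserStates subscribes to a user state's name-change dispatcher and immediately triggers a refresh of the widget's user list.
; If the widget is not yet valid, the refresh retries on a short timer, covering binds that arrive before BeginPlay creates it.
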(event EventBeginPlay
  (bind _returnvalue (Game|GetPlayerController 0))
  (bind _returnvalue_2 (UserInterface|CreateWidget "/Game/ShootingGame/Widget/Lobby/LobbyHudWidget.LobbyHudWidget_C"))
  (bind _output_get (Variables|Default|SetLobby _returnvalue_2))
  (UserInterface|Viewport|AddtoViewport _output_get 0)
  (Input|SetInputModeUIOnly _returnvalue 0 "DoNotLock")
  (Variables|/Script/Engine.PlayerController|SetbShowMouseCursor _returnvalue true))

(fn ConstructionScript)

(fn BindUserStates
  (params (UserStates :type BP%20Lobby%20Player%20States%20Object%20Reference))
  (EventDispatchers|BindEventtoEventDispatcherChangeName UserStates (EventDispatchers|CreateEvent :!event EventChangeName))
  (CallFunction|EventChangeName))

(fn EventChangeName
  (params (NewName :type String))
  (CallFunction|RFChangeName))

(fn RFChangeName
  (bind _lobby (Variables|Default|GetLobby))
  (Utilities|IsValid _lobby
    (:Is%20Valid
      (Default|UpdateUserList _lobby))
    (:Is%20Not%20Valid
      (Utilities|Time|SetTimerbyFunctionName 0 "RF_ChangeName" 0.1))))