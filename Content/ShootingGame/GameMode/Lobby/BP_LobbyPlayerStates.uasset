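; Lobby player state that holds each player's name and exposes changes to the lobby UI.
; On BeginPlay it registers itself with the local player's lobby HUD through BindUserStates, printing an error if the HUD cast fails.
; Name is a RepNotify variable set by SetName; its OnRep prints a debug message and fires a ChangeName dispatcher with the new value.
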(event EventBeginPlay
  (CallFunction|InitBind))

(fn ConstructionScript)

(fn SetName
  (params (Name :type String))
  (Variables|Default|SetName Name))

(fn InitBind
  (bind _asbp_lobby_hud (Utilities|Casting|CastToBP_LobbyHUD (HUD|GetHUD (Game|GetPlayerController 0)))
    (:then
      (Default|BindUserStates _asbp_lobby_hud self))
    (:CastFailed
      (Development|PrintString "LobbyHUD_Cast Fail" true true "(R=1.000000,G=0.025870,B=0.000000,A=1.000000)" 6e+01))))

(fn OnRepName
  (Development|PrintString (Utilities|String|Append "OnRepName" "   :   " (Variables|Default|GetName)) true true "(R=1.000000,G=0.216980,B=0.000000,A=1.000000)" 6e+01)
  (Default|CallEventDispatcherChangeName (Variables|Default|GetName)))