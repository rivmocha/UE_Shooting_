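; Shooting game HUD that creates and displays the main HUD widget and sets game-only input on BeginPlay.
; Update functions forward ammo, magazine, HP, armor and F-guide position and visibility to the widget.
; It binds local PlayerState HP and armor dispatchers; a failed cast sets a timer naming BindPlayerState, not itself.
; BindPlayerState hooks a given player's name, kill and death dispatchers to refresh the player list.
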(event EventBeginPlay
  (bind _returnvalue (Game|GetPlayerController 0))
  (bind _returnvalue_2 (UserInterface|CreateWidget "/Game/ShootingGame/Widget/SHootingHUDWidget.SHootingHUDWidget_C"))
  (bind _output_get (Variables|Default|SetHUDWidget _returnvalue_2))
  (UserInterface|Viewport|AddtoViewport _output_get 0)
  (CallFunction|BindMyPlayerState)
  (Input|SetInputModeGameOnly _returnvalue)
  (Variables|/Script/Engine.PlayerController|SetbShowMouseCursor _returnvalue false))

(fn ConstructionScript)

(fn UpdateAmmo
  (params (Ammo :type Integer))
  (Default|SetAmmo (Variables|Default|GetHUDWidget) Ammo))

(fn UpdateMag
  (params (Mag :type Integer))
  (Default|SetMag (Variables|Default|GetHUDWidget) Mag))

(fn UpdateHP
  (params (Cur%20HP :type Float%20%28single-precision%29) (Max%20Hp :type Float%20%28single-precision%29))
  (Default|SetHP (Variables|Default|GetHUDWidget) Cur%20HP Max%20Hp))

(fn UpdateGuideF
  (params (WorldLocation :type Vector))
  (Default|SetPositionGuideF (Variables|Default|GetHUDWidget) WorldLocation))

(fn SetVisibilityGuideF
  (params (InVisibility :type ESlateVisibility%20Enum :default "Visible"))
  (Default|SetVisibilityGuideF (Variables|Default|GetHUDWidget) InVisibility))

(fn UpdateArmor
  (params (CurHP :type Float%20%28single-precision%29) (MaxHP :type Float%20%28single-precision%29))
  (Default|SetArmor (Variables|Default|GetHUDWidget) CurHP MaxHP))

(fn BindMyPlayerState
  (bind _asbp_shooting_player_states (Utilities|Casting|CastToBP_ShootingPlayerStates (Variables|/Script/Engine.Controller|GetPlayerState (Game|GetPlayerController 0)))
    (:then
      (EventDispatchers|BindEventtoEventDispatcherHP _asbp_shooting_player_states (EventDispatchers|CreateEvent :!event UpdateHP))
      (EventDispatchers|BindEventtoEventDispatcherArmor _asbp_shooting_player_states (EventDispatchers|CreateEvent :!event UpdateArmor)))
    (:CastFailed
      (Utilities|Time|SetTimerbyFunctionName 0 "BindPlayerState" 0.1))))

(fn EventKill
  (params (Kill :type Integer))
  (CallFunction|UpdatePlayerList))

(fn UpdatePlayerList
  (bind _hudwidget (Variables|Default|GetHUDWidget))
  (Utilities|IsValid _hudwidget
    (:Is%20Valid
      (Default|UpdatePlayerList _hudwidget))
    (:Is%20Not%20Valid
      (Utilities|Time|SetTimerbyFunctionName 0 "UpdatePlayerList" 0.0))))

(fn BindPlayerState
  (params (Playerstate :type BP%20Shooting%20Player%20States%20Object%20Reference))
  (EventDispatchers|BindEventtoEventDispatcherChangeName Playerstate (EventDispatchers|CreateEvent :!event EventChangeName))
  (EventDispatchers|BindEventtoEventDispatcherKill Playerstate (EventDispatchers|CreateEvent :!event EventKill))
  (EventDispatchers|BindEventtoEventDispatcherDeath Playerstate (EventDispatchers|CreateEvent :!event EventDeath))
  (CallFunction|UpdatePlayerList))

(fn EventChangeName
  (params (Name :type String))
  (CallFunction|UpdatePlayerList))

(fn EventDeath
  (params (Death :type Integer))
  (CallFunction|UpdatePlayerList))